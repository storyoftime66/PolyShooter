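; Pooled projectile Blueprint for PolyShooter that leaves its behavior to its parent class.
; Tick only calls the parent, while the pool begin and end events call the parent and then print a debug message to trace pooling.
; Disconnected leftover nodes hold debug aids for drawing a box at the projectile and printing its location on simulated proxies.
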(event EventBeginPlay)

(event Collision|EventActorBeginOverlap
  (params (OtherActor :type Actor%20Object%20Reference)))

(event EventTick
  (params (DeltaSeconds :type Float%20%28single-precision%29))
  (|CallParentFunction DeltaSeconds))

(event EventOnPoolEnd
  (|CallParentFunction)
  (Development|PrintString "OnPoolEnd" true true "(R=1.000000,G=0.315328,B=0.000000,A=1.000000)"))

(event EventOnPoolBegin
  (|CallParentFunction)
  (Development|PrintString "OnPoolBegin" true true "(R=1.000000,G=0.315328,B=0.000000,A=1.000000)"))

(fn ConstructionScript)