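; Debug pawn that tests aligning a weapon's aim-down-sight socket with the camera by shifting the skeletal mesh.
; On BeginPlay it caches the camera's transform relative to that socket and the mesh's relative transform, then enables simulation after a short delay.
; Tick prints the offset and, while simulating, applies and prints the composed mesh transform.
; Possession by a player controller adds a debug crosshair widget.
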(event EventBeginPlay
  (Utilities|FlowControl|Sequence
    (:then_0
      (Variables|Default|SetAimTransformOffset (Math|Transform|MakeRelativeTransform (Transformation|GetWorldTransform (Variables|Default|GetCamera)) (Transformation|GetSocketTransform (Variables|Default|GetWeapon) "SOCKET_AimDownSight" "RTS_World")))
      (Variables|Default|SetOriginTransform (Transformation|GetRelativeTransform (Variables|Default|GetSkeletalMesh)))
      (Utilities|FlowControl|Delay 2.0)
      (Variables|Default|SetbSimulate true))))

(event Collision|EventActorBeginOverlap
  (params (OtherActor :type Actor%20Object%20Reference)))

(event EventTick
  (params (DeltaSeconds :type Float%20%28single-precision%29))
  (bind _aimtransformoffset (Variables|Default|GetAimTransformOffset))
  (bind _origintransform (Variables|Default|GetOriginTransform))
  (bind _returnvalue (Math|Transform|ComposeTransforms _origintransform _aimtransformoffset))
  (Utilities|FlowControl|Sequence
    (:then_0
      (Development|PrintString (Utilities|String|ToString(Transform) (Variables|Default|GetAimTransformOffset)) true true "(R=0.000000,G=0.660000,B=1.000000,A=1.000000)" 0.0))
    (:then_1
      (if (Variables|Default|GetbSimulate)
        (Transformation|SetRelativeTransform (Variables|Default|GetSkeletalMesh) _returnvalue false false)
        (Development|PrintString (Utilities|String|ToString(Transform) _returnvalue) true true "(R=0.000000,G=1.000000,B=0.028466,A=1.000000)" 0.0)))))

(event EventPossessed
  (params (NewController :type Controller%20Object%20Reference))
  (bind _as玩家控制器 (Utilities|Casting|CastToPlayerController NewController))
  (bind _returnvalue (UserInterface|CreateWidget "/Game/PolyShooter/Blueprints/UMG_CrosshairDebuger.UMG_CrosshairDebuger_C" _as玩家控制器))
  (UserInterface|Viewport|AddtoViewport _returnvalue 0))

(fn ConstructionScript)